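; Player-controllable tank pawn Blueprint that wires up the tank's parts and input.
; On BeginPlay it registers barrel and turret references and gives both tracks to TankMovementComponent, which receives move and turn intents from input axes.
; Camera look splits yaw onto an azimuth gimbal and pitch onto the spring arm to keep rotation smooth.
; It also handles firing and toggles a lazily created pause menu, switching cursor and input mode.
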(event `self.ReceiveBeginPlay`
  (`self.SetBarrelReference` (`self.TankBarrel`))
  (`self.SetTurretReference` (`self.TankTurret`))
  (`TankMovementComponent.Initialize` (`self.TankMovementComponent`) (`self.RTrack`) (`self.LTrack`)))

(event `InputAxis|Move Forward`
  (params (AxisValue :type "Float (single-precision)"))
  ;[1 1 1] Controlling Tank Track Movement
  (`TankMovementComponent.IntendMoveForward` (`self.TankMovementComponent`) AxisValue))

(event `InputAxis|AltitudeAxis`
  (params (AxisValue :type "Float (single-precision)"))
  ;[1 1 1] Controlling Camera View Axis
  (`SceneComponent.K2_AddLocalRotation` (`self.SpringArm`) (`KismetMathLibrary.MakeRotator` 0.0 AxisValue) false false))

(event `InputAxis|Turn Right`
  (params (AxisValue :type "Float (single-precision)"))
  ;[1 1 1] Controlling Tank Track Movement
  (`TankMovementComponent.IntendRotateRight` (`self.TankMovementComponent`) AxisValue))

(event `InputAxis|Turn Left`
  (params (AxisValue :type "Float (single-precision)"))
  ;[1 1 1] Controlling Tank Track Movement
  (`TankMovementComponent.IntendRotateLeft` (`self.TankMovementComponent`) AxisValue))

(event `InputAxis|AzimuthAxis`
  (params (AxisValue :type "Float (single-precision)"))
  ;[1 1 1] Controlling Camera View Axis
  ;;[1 1 1] Prevents staggering of rotations
  (`SceneComponent.K2_AddLocalRotation` (`self.AzimuthGimbal`) (`KismetMathLibrary.MakeRotator` 0.0 0.0 AxisValue) false false))

(event `InputAxis|Move Backward`
  (params (AxisValue :type "Float (single-precision)"))
  ;[1 1 1] Controlling Tank Track Movement
  (`TankMovementComponent.IntendMoveBackward` (`self.TankMovementComponent`) AxisValue))

(event `InputAction|Fire`
  (params (Key :type "Key Structure"))
  ;[1 1 1] Controlling Camera View Axis
  (:`Pressed`
    (`self.Fire`)))

(event `InputAction|PauseGame` :paused true
  (params (Key :type "Key Structure"))
  (bind _returnvalue (`GameplayStatics.GetPlayerController` 0))
  (bind _pause_menu_ref (`self.Pause Menu REF`))
  ;[1 1 1] Pause / Unpause game
  (:`Pressed`
    (`/Engine/EditorBlueprintResources/StandardMacros.IsValid` null
      (:`Is Valid`
        _)
      (:`Is Not Valid`
        (bind _returnvalue_2 (`|CreateWidget` "/Game/UI/GameMenu_BP.GameMenu_BP_C"))
        (set `self.Pause Menu REF` _returnvalue_2)))
    (if (`GameplayStatics.IsGamePaused`)
      (`Widget.RemoveFromParent` _pause_menu_ref)
      (`GameplayStatics.SetGamePaused` false)
      (set `PlayerController.bShowMouseCursor` false _returnvalue)
      (`WidgetBlueprintLibrary.SetInputMode_GameOnly` _returnvalue)
      (else
        (`UserWidget.AddToViewport` _pause_menu_ref 0)
        (`GameplayStatics.SetGamePaused` true)
        (set `PlayerController.bShowMouseCursor` true _returnvalue)
        (`WidgetBlueprintLibrary.SetInputMode_GameAndUIEx` _returnvalue _pause_menu_ref "LockInFullscreen" false)))))

(fn `UserConstructionScript`)