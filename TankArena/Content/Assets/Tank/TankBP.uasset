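; Player-controllable tank Blueprint that wires its components together and routes input to movement, camera and firing.
; On BeginPlay it passes barrel and turret references to the tank and initializes the movement component with both tracks.
; Move and turn axes send intents to TankMovementComponent, and the Fire action calls Fire.
; Camera yaw rotates an azimuth gimbal while pitch rotates the spring arm, separating the axes to keep rotation smooth.
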(event `self.ReceiveBeginPlay`
  (`self.SetBarrelReference` (`self.TankBarrel`))
  (`self.SetTurretReference` (`self.TankTurret`))
  (`TankMovementComponent.Initialize` (`self.TankMovementComponent`) (`self.RTrack`) (`self.LTrack`)))

(event `InputAxis|Move Forward`
  (params (AxisValue :type "Float (single-precision)"))
  ;[1 1 1] Controlling Tank Track Movement
  (`TankMovementComponent.IntendMoveForward` (`self.TankMovementComponent`) AxisValue))

(event `InputAxis|AltitudeAxis`
  (params (AxisValue :type "Float (single-precision)"))
  ;[1 1 1] Controlling Camera View Axis
  (`SceneComponent.K2_AddLocalRotation` (`self.SpringArm`) (`KismetMathLibrary.MakeRotator` 0.0 AxisValue) false false))

(event `InputAxis|Turn Right`
  (params (AxisValue :type "Float (single-precision)"))
  ;[1 1 1] Controlling Tank Track Movement
  (`TankMovementComponent.IntendRotateRight` (`self.TankMovementComponent`) AxisValue))

(event `InputAxis|Turn Left`
  (params (AxisValue :type "Float (single-precision)"))
  ;[1 1 1] Controlling Tank Track Movement
  (`TankMovementComponent.IntendRotateLeft` (`self.TankMovementComponent`) AxisValue))

(event `InputAxis|AzimuthAxis`
  (params (AxisValue :type "Float (single-precision)"))
  ;[1 1 1] Controlling Camera View Axis
  ;;[1 1 1] Prevents staggering of rotations
  (`SceneComponent.K2_AddLocalRotation` (`self.AzimuthGimbal`) (`KismetMathLibrary.MakeRotator` 0.0 0.0 AxisValue) false false))

(event `InputAxis|Move Backward`
  (params (AxisValue :type "Float (single-precision)"))
  ;[1 1 1] Controlling Tank Track Movement
  (`TankMovementComponent.IntendMoveBackward` (`self.TankMovementComponent`) AxisValue))

(event `InputAction|Fire`
  (params (Key :type "Key Structure"))
  ;[1 1 1] Controlling Camera View Axis
  (:`Pressed`
    (`self.Fire`)))

(fn `UserConstructionScript`)